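; Creature actor that takes its stats from CreatureType and dies of starvation as its Hunger runs out.
; BeginPlay copies health, diet and food points from CreatureType, the latter into its ResourceComponent, and applies the creature material to the Cube.
; Tick uses a Delay to decrement Hunger at the type's interval, destroying the actor once it reaches zero.
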(event EventBeginPlay
  (bind _creaturetype (Variables|Default|GetCreatureType))
  (Variables|Default|SetHealth (Variables|/Game/Blueprints/CreatureDataAsset.CreatureDataAsset_C|GetHealth _creaturetype))
  (Rendering|Material|SetMaterial (Variables|Default|GetCube) 0 (Variables|/Game/Blueprints/CreatureDataAsset.CreatureDataAsset_C|GetCreatureMaterial _creaturetype))
  (Variables|/Game/Blueprints/ResourceComponent.ResourceComponent_C|SetFoodPoints (Variables|Default|GetResourceComponent) (Variables|/Game/Blueprints/CreatureDataAsset.CreatureDataAsset_C|GetFoodPoints _creaturetype))
  (Variables|Default|SetDiet (Variables|/Game/Blueprints/CreatureDataAsset.CreatureDataAsset_C|GetDiet _creaturetype)))

(event Collision|EventActorBeginOverlap
  (params (OtherActor :type Actor%20Object%20Reference)))

(event EventTick
  (params (DeltaSeconds :type Float%20%28single-precision%29))
  (Utilities|FlowControl|Sequence
    (:then_0
      (Utilities|FlowControl|Delay (Variables|/Game/Blueprints/CreatureDataAsset.CreatureDataAsset_C|GetTimeBetweenHungerIncrease (Variables|Default|GetCreatureType)))
      (bind _result (Math|Integer|DecrementInt (Variables|Default|GetHunger))
        (:%20%20
          (if (<= _result 0)
            (Actor|DestroyActor)))))))

(fn ConstructionScript)